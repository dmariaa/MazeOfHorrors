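; Actor that builds a square grid maze of floor and wall mesh instances in its Construction Script.
; InitMaze creates MazeCell objects and connects each to its four neighbours.
; GenerateMaze carves passages with a stack-based randomized depth-first backtracker, linking cells both ways.
; DrawMaze adds a scaled floor instance per cell and a wall on every side without a linked neighbour, so interior walls are added from both cells.
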(event EventBeginPlay)

(event Collision|EventActorBeginOverlap
  (params (OtherActor :type Actor%20Object%20Reference)))

(event EventTick
  (params (DeltaSeconds :type Float%20%28single-precision%29)))

(fn ConstructionScript
  (CallFunction|InitMaze)
  (CallFunction|GenerateMaze)
  (CallFunction|DrawMaze))

(fn InitMaze
  (bind _size (Variables|Default|GetSize))
  ;[1 1 1] Clear Maze
  (Utilities|Array|Clear (Variables|Default|GetMaze))
  ;[1 1 1] Resize Maze
  (Utilities|Array|Resize (Variables|Default|GetMaze) (* _size _size))
  (for (_ _array_index) (Variables|Default|GetMaze)
    (bind _returnvalue (Game|ConstructObjectfromClass "/Game/MazeGenerator/Blueprints/MazeCell.MazeCell_C" self))
    (bind _position (CallFunction|IndextoPosition _array_index))
    (Utilities|Array|SetArrayElem (Variables|Default|GetMaze) _array_index _returnvalue)
    (Variables|/Game/MazeGenerator/Blueprints/MazeCell.MazeCell_C|SetPosition _returnvalue _position))
  (for _array_element (Variables|Default|GetMaze)
    (bind _cell (CallFunction|GetCellat (+ (Variables|/Game/MazeGenerator/Blueprints/MazeCell.MazeCell_C|GetPosition _array_element) "(X=0.000000,Y=-1.000000)")))
    (Variables|/Game/MazeGenerator/Blueprints/MazeCell.MazeCell_C|SetNorth _array_element _cell)
    (bind _cell_2 (CallFunction|GetCellat (+ (Variables|/Game/MazeGenerator/Blueprints/MazeCell.MazeCell_C|GetPosition _array_element) "(X=0.000000,Y=1.000000)")))
    (Variables|/Game/MazeGenerator/Blueprints/MazeCell.MazeCell_C|SetSouth _array_element _cell_2)
    (bind _cell_3 (CallFunction|GetCellat (+ (Variables|/Game/MazeGenerator/Blueprints/MazeCell.MazeCell_C|GetPosition _array_element) "(X=1.000000,Y=0.000000)")))
    (Variables|/Game/MazeGenerator/Blueprints/MazeCell.MazeCell_C|SetEast _array_element _cell_3)
    (bind _cell_4 (CallFunction|GetCellat (+ (Variables|/Game/MazeGenerator/Blueprints/MazeCell.MazeCell_C|GetPosition _array_element) "(X=-1.000000,Y=0.000000)")))
    (Variables|/Game/MazeGenerator/Blueprints/MazeCell.MazeCell_C|SetWest _array_element _cell_4)))

(fn GetCellIndex
  (params (Cell :type Maze%20Cell%20Object%20Reference))
  (bind _index (CallFunction|PositiontoIndex (Variables|/Game/MazeGenerator/Blueprints/MazeCell.MazeCell_C|GetPosition Cell)))
  (return _index))

(fn GetCellat
  (params (Position :type Vector%202D%20Structure))
  (bind (_x _y) (Math|Vector2D|BreakVector2D Position))
  (bind _size (Variables|Default|GetSize))
  (if (Math|Boolean|ORBoolean (< _x 0.0) (>= _x (Math|Conversions|ToFloat(Integer) _size)) (>= _y (Math|Conversions|ToFloat(Integer) _size)) (< _y 0.0))
    (return (LocalVariables|GetNullCell))
    (else
      (bind _index (CallFunction|PositiontoIndex Position))
      (return (Utilities|Array|Get(acopy) (Variables|Default|GetMaze) _index)))))

(fn IndextoPosition
  (params (Index :type Integer))
  (bind _size (Variables|Default|GetSize))
  (return (Math|Vector2D|MakeVector2D (Math|Conversions|ToFloat(Integer) (Math|Integer|%(Integer) Index _size)) (Math|Conversions|ToFloat(Integer) (/ Index _size)))))

(fn PositiontoIndex
  (params (Position :type Vector%202D%20Structure))
  (bind (_x _y) (Math|Vector2D|BreakVector2D Position))
  (return (Math|Float|Truncate (+ _x (* (Variables|Default|GetSize) _y)))))

(fn GenerateMaze
  (bind _stack (LocalVariables|GetStack))
  (bind _stack_2 (LocalVariables|GetStack))
  (Utilities|Array|Add (LocalVariables|GetStack) (Utilities|Array|Get(acopy) (Variables|Default|GetMaze)))
  (while (Utilities|Array|IsValidIndex _stack)
    (bind _output_get (LocalVariables|SetCurrent (Utilities|Array|Get(acopy) _stack (Utilities|Array|LastIndex _stack))))
    (bind (_neighbour _foundone) (Default|GetRandomEmptyNeighbour _output_get))
    (if _foundone
      (Default|Link _output_get _neighbour true)
      (Utilities|Array|Add (LocalVariables|GetStack) _neighbour)
      (else
        (Utilities|Array|RemoveIndex _stack_2 (Utilities|Array|LastIndex _stack_2))))))

(fn DrawMaze
  (for _array_element (Variables|Default|GetMaze)
    (CallFunction|BuildFloor _array_element)
    (CallFunction|BuildWall _array_element (Variables|/Game/MazeGenerator/Blueprints/MazeCell.MazeCell_C|GetNorth _array_element) "NewEnumerator0")
    (CallFunction|BuildWall _array_element (Variables|/Game/MazeGenerator/Blueprints/MazeCell.MazeCell_C|GetSouth _array_element) "NewEnumerator1")
    (CallFunction|BuildWall _array_element (Variables|/Game/MazeGenerator/Blueprints/MazeCell.MazeCell_C|GetEast _array_element) "NewEnumerator2")
    (CallFunction|BuildWall _array_element (Variables|/Game/MazeGenerator/Blueprints/MazeCell.MazeCell_C|GetWest _array_element) "NewEnumerator3")))

(fn BuildWall
  (params (Current :type Maze%20Cell%20Object%20Reference) (Wall :type Maze%20Cell%20Object%20Reference) (WallPosition :type Walls%20Enum :default "NewEnumerator0"))
  (bind _blocksize (Variables|Default|GetBlockSize))
  (bind _blocksize_2 (Variables|Default|GetBlockSize))
  (bind _blocksize_3 (Variables|Default|GetBlockSize))
  (bind _blocksize_4 (Variables|Default|GetBlockSize))
  (bind _blocksize_5 (Variables|Default|GetBlockSize))
  (bind _blocksize_6 (Variables|Default|GetBlockSize))
  (bind _blocksize_7 (Variables|Default|GetBlockSize))
  (bind _blocksize_8 (Variables|Default|GetBlockSize))
  (bind _returnvalue (* _blocksize_8 1e+02))
  (bind _returnvalue_2 (* _blocksize_4 1e+02))
  (bind _returnvalue_3 (* _blocksize_6 1e+02))
  (bind _returnvalue_4 (* _blocksize_2 1e+02))
  (bind _position (Variables|/Game/MazeGenerator/Blueprints/MazeCell.MazeCell_C|GetPosition Current))
  (bind _position_2 (Variables|/Game/MazeGenerator/Blueprints/MazeCell.MazeCell_C|GetPosition Current))
  (bind _position_3 (Variables|/Game/MazeGenerator/Blueprints/MazeCell.MazeCell_C|GetPosition Current))
  (bind _position_4 (Variables|/Game/MazeGenerator/Blueprints/MazeCell.MazeCell_C|GetPosition Current))
  (bind _returnvalue_5 (Math|Conversions|ToVector(Vector2D) _position))
  (bind _returnvalue_6 (Math|Conversions|ToVector(Vector2D) _position_2))
  (bind _returnvalue_7 (Math|Conversions|ToVector(Vector2D) _position_3))
  (bind _returnvalue_8 (Math|Conversions|ToVector(Vector2D) _position_4))
  (bind _returnvalue_9 (* _returnvalue_4 -0.5))
  (bind _returnvalue_10 (* _returnvalue_2 0.5))
  (bind _returnvalue_11 (* _returnvalue_2 0.5))
  (bind _returnvalue_12 (* _returnvalue_3 0.5))
  (bind _returnvalue_13 (* _returnvalue_3 0.5))
  (bind _returnvalue_14 (* _returnvalue -0.5))
  (bind _returnvalue_15 (* _returnvalue 0.5))
  (bind _returnvalue_16 (* _returnvalue_4 0.5))
  (bind _returnvalue_17 (* _returnvalue_5 _returnvalue_4))
  (bind _returnvalue_18 (* _returnvalue_6 _returnvalue_2))
  (bind _returnvalue_19 (* _returnvalue_7 _returnvalue_3))
  (bind _returnvalue_20 (* _returnvalue_8 _returnvalue))
  (bind _returnvalue_21 (+ _returnvalue_18 (Math|Vector|MakeVector 0.0 _returnvalue_11 _returnvalue_10)))
  (bind _returnvalue_22 (+ _returnvalue_19 (Math|Vector|MakeVector _returnvalue_13 0.0 _returnvalue_12)))
  (bind _returnvalue_23 (+ _returnvalue_20 (Math|Vector|MakeVector _returnvalue_14 0.0 _returnvalue_15)))
  (bind _returnvalue_24 (+ _returnvalue_17 (Math|Vector|MakeVector 0.0 _returnvalue_9 _returnvalue_16)))
  (if (not (and (.ReturnValue (Utilities|Map|Find (Variables|/Game/MazeGenerator/Blueprints/MazeCell.MazeCell_C|GetLinks Current) Wall)) (Utilities|IsValid Wall)))
    (switch Utilities|FlowControl|Switch|SwitchonWalls WallPosition
      (:NewEnumerator0
        (bind _output_get (LocalVariables|SetBlockTransform (Math|Transform|MakeTransform (Math|Vector|MakeVector (.x _returnvalue_24) (.y _returnvalue_24) (.z _returnvalue_24)) "0, 0, 0" (Math|Vector|MakeVector _blocksize_7 0.2 _blocksize_7))))
        (Components|InstancedStaticMesh|AddInstance (Variables|Default|GetWallMesh) _output_get))
      (:NewEnumerator1
        (bind _output_get_2 (LocalVariables|SetBlockTransform (Math|Transform|MakeTransform (Math|Vector|MakeVector (.x _returnvalue_21) (.y _returnvalue_21) (.z _returnvalue_21)) "0, 0, 0" (Math|Vector|MakeVector _blocksize_3 0.2 _blocksize_3))))
        (Components|InstancedStaticMesh|AddInstance (Variables|Default|GetWallMesh) _output_get_2))
      (:NewEnumerator2
        (bind _output_get_3 (LocalVariables|SetBlockTransform (Math|Transform|MakeTransform (Math|Vector|MakeVector (.x _returnvalue_22) (.y _returnvalue_22) (.z _returnvalue_22)) "0, 0, 0" (Math|Vector|MakeVector 0.2 _blocksize_5 _blocksize_5))))
        (Components|InstancedStaticMesh|AddInstance (Variables|Default|GetWallMesh) _output_get_3))
      (:NewEnumerator3
        (bind _output_get_4 (LocalVariables|SetBlockTransform (Math|Transform|MakeTransform (Math|Vector|MakeVector (.x _returnvalue_23) (.y _returnvalue_23) (.z _returnvalue_23)) "0, 0, 0" (Math|Vector|MakeVector 0.2 _blocksize _blocksize))))
        (Components|InstancedStaticMesh|AddInstance (Variables|Default|GetWallMesh) _output_get_4)))))

(fn BuildFloor
  (params (self2 :type Maze%20Cell%20Object%20Reference))
  (bind _position (Variables|/Game/MazeGenerator/Blueprints/MazeCell.MazeCell_C|GetPosition self2))
  (bind _blocksize (Variables|Default|GetBlockSize))
  (Components|InstancedStaticMesh|AddInstance (Variables|Default|GetFloorMesh) (Math|Transform|MakeTransform (* (Math|Vector|MakeVector (.x _position) (.y _position) 0.0) (* 1e+02 _blocksize)) "0, 0, 0" (Math|Vector|MakeVector _blocksize _blocksize 0.2))))