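; Unfinished grid maze generator, apparently an older version, that builds a Size by Size array of cell structs on BeginPlay.
; Each cell stores its grid position, with outer edges marked -1 so the neighbour search skips them.
; GenerateMaze sketches a stack-based depth-first walk using random neighbours, but is never called and only handles popping dead ends.
; LinkCells is an empty stub with unconnected direction comparisons.
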(event EventBeginPlay
  (CallFunction|InitializeMazeArray))

(event Collision|EventActorBeginOverlap
  (params (OtherActor :type Actor%20Object%20Reference)))

(event EventTick
  (params (DeltaSeconds :type Float%20%28single-precision%29)))

(fn ConstructionScript)

(fn InitializeMazeArray
  (bind _size (Variables|Default|GetSize))
  (bind _size_2 (Variables|Default|GetSize))
  (bind _returnvalue (- _size_2 1))
  ;[1 1 1] Clear Cell Array
  (Utilities|Array|Clear (Variables|Default|GetMaze))
  ;[1 1 1] Resize Cell Array
  (Utilities|Array|Resize (Variables|Default|GetMaze) (* _size _size))
  ;[1 1 1] Populate Cell Array
  (for (_ _array_index) (Variables|Default|GetMaze)
    (Utilities|Struct|SetmembersinStructMazeCell (Utilities|Array|Get(acopy) (Variables|Default|GetMaze) _array_index) (Math|Vector2D|MakeVector2D (Math|Conversions|ToFloat(Integer) (Math|Integer|%(Integer) _array_index _size_2)) (Math|Conversions|ToFloat(Integer) (/ _array_index _size_2))))
    (if (== (/ _array_index _size_2) 0)
      (Utilities|Struct|SetmembersinStructMazeCell (Utilities|Array|Get(acopy) (Variables|Default|GetMaze) _array_index) -1))
    (if (== (/ _array_index _size_2) _returnvalue)
      (Utilities|Struct|SetmembersinStructMazeCell (Utilities|Array|Get(acopy) (Variables|Default|GetMaze) _array_index) -1))
    (if (== (Math|Integer|%(Integer) _array_index _size_2) 0)
      (Utilities|Struct|SetmembersinStructMazeCell (Utilities|Array|Get(acopy) (Variables|Default|GetMaze) _array_index) -1))
    (if (== (Math|Integer|%(Integer) _array_index _size_2) _returnvalue)
      (Utilities|Struct|SetmembersinStructMazeCell (Utilities|Array|Get(acopy) (Variables|Default|GetMaze) _array_index) -1))))

(fn GenerateMaze
  (Utilities|Array|Insert (LocalVariables|GetStack) (Utilities|Array|Get(acopy) (Variables|Default|GetMaze)))
  (while (> (Utilities|Array|Length (LocalVariables|GetStack)) 0)
    (bind _output_get (LocalVariables|SetCurrent (Utilities|Array|Get(acopy) (LocalVariables|GetStack))))
    (bind _found (CallFunction|GetAleatoryValidNeighbour _output_get))
    (if (not _found)
      (Utilities|Array|RemoveIndex (LocalVariables|GetStack)) ; Stack POP
    )))

(fn GetAleatoryValidNeighbour
  (params (Current :type Struct%20Maze%20Cell%20Structure))
  (bind (_position _north _south _east _west) (Utilities|Struct|BreakStructMazeCell Current))
  (bind _neighbours (LocalVariables|GetNeighbours))
  (bind _neighbours_2 (LocalVariables|GetNeighbours))
  ;[1 1 1] Add North Cell to Neighbours
  (if (== _north 0)
    (bind _cell (CallFunction|GetMaceCell (+ _position "(X=0.000000,Y=-1.000000)")))
    (Utilities|Array|Add (LocalVariables|GetNeighbours) _cell))
  ;[1 1 1] Add South Cell to Neighbours
  (if (== _south 0)
    (bind _cell_2 (CallFunction|GetMaceCell (+ _position "(X=0.000000,Y=1.000000)")))
    (Utilities|Array|Add (LocalVariables|GetNeighbours) _cell_2))
  ;[1 1 1] Add East Cell to Neighbours
  (if (== _east 0)
    (bind _cell_3 (CallFunction|GetMaceCell (+ _position "(X=1.000000,Y=0.000000)")))
    (Utilities|Array|Add (LocalVariables|GetNeighbours) _cell_3))
  ;[1 1 1] Add West Cell to Neighbours
  (if (== _west 0)
    (bind _cell_4 (CallFunction|GetMaceCell (+ _position "(X=-1.000000,Y=0.000000)")))
    (Utilities|Array|Add _neighbours_2 _cell_4))
  (Utilities|Array|Shuffle _neighbours_2)
  (if (Utilities|Array|IsValidIndex _neighbours)
    (return (Utilities|Array|Get(acopy) _neighbours) true)
    (else
      (return "" false))))

(fn GetMaceCell
  (params (Position :type Vector%202D%20Structure))
  (bind (_x _y) (Math|Vector2D|BreakVector2D Position))
  (return (Utilities|Array|Get(acopy) (Variables|Default|GetMaze) (Math|Float|Truncate (+ _x (* (Variables|Default|GetSize) _y))))))

(fn LinkCells
  (params (Current :type Struct%20Maze%20Cell%20Structure) (Linked :type Struct%20Maze%20Cell%20Structure)))