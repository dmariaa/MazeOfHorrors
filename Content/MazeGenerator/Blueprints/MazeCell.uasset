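; MazeCell represents one cell in a generated maze, holding references to its four compass neighbours and a map of the cells it links to.
; Link and UnLink edit that map, optionally mirroring the change on the other cell through a non-recursing call.
; An empty link map marks a cell as unvisited, so GetRandomEmptyNeighbour shuffles the valid unlinked neighbours and returns one, or reports none found.
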(fn GetRandomEmptyNeighbour
  (bind _south (Variables|Default|GetSouth))
  (bind _east (Variables|Default|GetEast))
  (bind _west (Variables|Default|GetWest))
  (bind _north (Variables|Default|GetNorth))
  ;[1 1 1] Collect North Cell If Valid and Not Visited (links empty)
  (Utilities|IsValid _north
    (:Is%20Valid
      (if (== (Utilities|Map|Length (Variables|MazeCell_C|GetLinks _north)) 0)
        (Utilities|Array|Add (LocalVariables|GetValidNeighbours) _north)))
    (:Is%20Not%20Valid
      _))
  ;[1 1 1] Collect South Cell If Valid and Not Visited (links empty)
  (Utilities|IsValid _south
    (:Is%20Valid
      (if (== (Utilities|Map|Length (Variables|MazeCell_C|GetLinks _south)) 0)
        (Utilities|Array|Add (LocalVariables|GetValidNeighbours) _south)))
    (:Is%20Not%20Valid
      _))
  ;[1 1 1] Collect East Cell If Valid and Not Visited (links empty)
  (Utilities|IsValid _east
    (:Is%20Valid
      (if (== (Utilities|Map|Length (Variables|MazeCell_C|GetLinks _east)) 0)
        (Utilities|Array|Add (LocalVariables|GetValidNeighbours) _east)))
    (:Is%20Not%20Valid
      _))
  ;[1 1 1] Collect West Cell If Valid and Not Visited (links empty)
  (Utilities|IsValid _west
    (:Is%20Valid
      (if (== (Utilities|Map|Length (Variables|MazeCell_C|GetLinks _west)) 0)
        (Utilities|Array|Add (LocalVariables|GetValidNeighbours) _west)))
    (:Is%20Not%20Valid
      _))
  ;[1 1 1] Return Cell or null
  (if (Utilities|Array|IsValidIndex (LocalVariables|GetValidNeighbours))
    (Utilities|Array|Shuffle (LocalVariables|GetValidNeighbours))
    (return (Utilities|Array|Get(acopy) (LocalVariables|GetValidNeighbours)) true)
    (else
      (return 0 false))))

(fn Link
  (params (Cell :type Maze%20Cell%20Object%20Reference) (Bidirectional :type Boolean))
  (Utilities|Map|Add (Variables|Default|GetLinks) Cell true)
  (if Bidirectional
    (CallFunction|Link Cell self false)))

(fn UnLink
  (params (Cell :type Maze%20Cell%20Object%20Reference) (Bidirectional :type Boolean))
  (Utilities|Map|Remove (Variables|Default|GetLinks) Cell)
  (if Bidirectional
    (CallFunction|UnLink Cell self false)))